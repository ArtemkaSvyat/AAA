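; Neuro actor that builds a vertical ring of InteractWidget components and reveals evenly spaced ones as answer slots for the current task.
; Start creates and orients the widgets, then reads the NeuroData row for the PC's TaskNum to set the answer count and advance TaskNum.
; BeginPlay registers the actor with Neuro_PC.
; MoveToDestroy plays the visible widgets' disappear animation while a looping timer pushes components outward, then destroys the actor.
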(event `Start`
  (bind _radius (`self.Radius`))
  (`KismetArrayLibrary.Array_Clear` (`self.AddedChildren`))
  (`KismetArrayLibrary.Array_Clear` (`self.AddedWidget`))
  (for _index (range 1 (+ (`self.Sides`) 1))
    (bind _returnvalue (`AddComponent|NODE_AddWidgetComponent-2`))
    (`KismetArrayLibrary.Array_Add` (`self.AddedChildren`) _returnvalue)
    (bind _returnvalue_2 (`|GenericCreateObject` "/Game/NeuroTestMap/InteractWidget.InteractWidget_C" self))
    (`WidgetComponent.SetWidget` _returnvalue _returnvalue_2)
    (`KismetArrayLibrary.Array_Add` (`self.AddedWidget`) _returnvalue_2)
    (bind _returnvalue_3 (* (/ 360.0 (`KismetMathLibrary.Conv_IntToDouble` (`self.Sides`))) (`KismetMathLibrary.Conv_IntToDouble` _index)))
    (`SceneComponent.K2_SetRelativeLocation` _returnvalue (`KismetMathLibrary.MakeVector` (* (`KismetMathLibrary.DegCos` _returnvalue_3) _radius) 0.0 (* (`KismetMathLibrary.DegSin` _returnvalue_3) _radius)) false false)
    (bind _returnvalue_4 (- _returnvalue_3 180.0))
    (`SceneComponent.K2_SetRelativeRotation` _returnvalue (`KismetMathLibrary.MakeRotator` (`KismetMathLibrary.SelectFloat` 0.0 180.0 (`KismetMathLibrary.InRange_FloatFloat` _returnvalue_4 -90.0 90.0)) _returnvalue_4) false false))
  (bind _returnvalue_5 (`|GetDataTableRow` "/Game/NeuroTestMap/NeuroData.NeuroData" (`KismetStringLibrary.Conv_StringToName` (`KismetStringLibrary.Conv_IntToString` (`/Game/NeuroTestMap/Neuro_PC.TaskNum` (`self.PC`)))))
    (:`then`
      (`self.SetAnswers` (`.Amount_8_E8BCE0C14FC2038075819398D791253B` (break `/Game/NeuroTestMap/NeuroStruct` _returnvalue_5))))))

(event `self.ReceiveBeginPlay`
  (bind _asneuro_pc (cast `/Game/NeuroTestMap/Neuro_PC` (`GameplayStatics.GetPlayerController` 0)))
  (set `self.PC` _asneuro_pc)
  (set `/Game/NeuroTestMap/Neuro_PC.NeuroActor` self (`self.PC`)))

(event `MoveToDestroy`
  (bind _returnvalue (`KismetSystemLibrary.K2_SetTimer` null "DestroyActorWidget" 0.01 true))
  (for _array_element (`self.AddedWidget`)
    (if (`|EnumEquality` (`Widget.GetVisibility` _array_element) "SelfHitTestInvisible")
      (`UserWidget.PlayAnimationForward` _array_element (`/Game/NeuroTestMap/InteractWidget.Dissapear` _array_element) 1.0 false)))
  (`KismetSystemLibrary.Delay` 2.0)
  (`KismetSystemLibrary.K2_ClearAndInvalidateTimerHandle` _returnvalue)
  (`self.K2_DestroyActor`))

(fn `DestroyActorWidget`
  (for _array_element (`self.AddedChildren`)
    (`SceneComponent.K2_AddRelativeLocation` _array_element (* (`SceneComponent.GetForwardVector` _array_element) -0.75) false false)))

(fn `SetAnswers`
  (params (AmountOfAnswers :type Integer))
  (locals (Step :type Integer :default 0))
  (set `local.Step` (/ (`self.Sides`) AmountOfAnswers))
  (for _index (range 1 (+ AmountOfAnswers 1))
    (bind _returnvalue (- (* _index (`local.Step`)) 1))
    (`Widget.SetVisibility` (`|GetArrayItem` (`self.AddedWidget`) _returnvalue) "SelfHitTestInvisible")
    (`KismetSystemLibrary.PrintString` (`KismetStringLibrary.Conv_IntToString` _returnvalue)))
  (set `/Game/NeuroTestMap/Neuro_PC.TaskNum` (+ (`/Game/NeuroTestMap/Neuro_PC.TaskNum` (`self.PC`)) AmountOfAnswers 1) (`self.PC`)))

(fn `UserConstructionScript`)